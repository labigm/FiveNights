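; BP_LightSwitch is a walk-over switch that dims or brightens the ceiling bar lights in the Dinner level.
; Each time a FirstPersonCharacter begins overlapping it, it flips a DimLights flag.
; Every tick, it finds all BP_CeilingBarLightDinner actors and calls their DimLights with a negative or positive amount according to that flag.
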(event `self.ReceiveActorBeginOverlap`
  (params (OtherActor :type "Actor Object Reference"))
  (cast `/Game/FirstPersonBP/Blueprints/FirstPersonCharacter` OtherActor)
  (set `self.DimLights?` (not (`self.DimLights?`))))

(event `self.ReceiveTick`
  (params (DeltaSeconds :type "Float (single-precision)"))
  (if (`self.DimLights?`)
    (`self.DimLights`)
    (else
      (`self.BrightLights`))))

(fn `BrightLights`
  (bind _outactors (`GameplayStatics.GetAllActorsOfClass` "/Game/Playground/Blueprints/FNF/Dinner/BP_CeilingBarLightDinner.BP_CeilingBarLightDinner_C"))
  (for _array_element _outactors
    (`/Game/Playground/Blueprints/FNF/Dinner/BP_CeilingBarLightDinner.Dim Lights` _array_element 100.0)))

(fn `DimLights`
  (bind _outactors (`GameplayStatics.GetAllActorsOfClass` "/Game/Playground/Blueprints/FNF/Dinner/BP_CeilingBarLightDinner.BP_CeilingBarLightDinner_C"))
  (for _array_element _outactors
    (`/Game/Playground/Blueprints/FNF/Dinner/BP_CeilingBarLightDinner.Dim Lights` _array_element -100.0)))

(fn `UserConstructionScript`)