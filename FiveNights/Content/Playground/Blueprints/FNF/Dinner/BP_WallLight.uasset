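; BP_WallLight is a wall light that continuously pulses its brightness over time.
; The construction script applies Brightness, Color and cone angles to PointLight2 and stores the starting brightness as MaxBrightness.
; Each Tick, Blink accumulates delta time and sets Brightness to the absolute sine scaled by MaxBrightness.
; Tick then applies that as intensity, fading smoothly between dark and full.
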(event `self.ReceiveTick`
  (params (DeltaSeconds :type "Float (single-precision)"))
  (`self.Blink` DeltaSeconds)
  (`LightComponent.SetIntensity` (`self.PointLight2`) (`self.Brightness`)))

(fn `Blink`
  (params (delta :type "Float (double-precision)"))
  (bind _output_get (set `self.Cumulative` (+ delta (`self.Cumulative`))))
  (bind _returnvalue (`KismetMathLibrary.Sin` _output_get))
  (if (> _returnvalue 0.0)
    (set `self.Brightness` (`KismetMathLibrary.FClamp` (* _returnvalue (`self.MaxBrightness`)) 0.0 (`self.MaxBrightness`)))
    (else
      (set `self.Brightness` (`KismetMathLibrary.FClamp` (* (* _returnvalue -1.0) (`self.MaxBrightness`)) 0.0 (`self.MaxBrightness`))))))

(fn `UserConstructionScript`
  (bind _pointlight2 (`self.PointLight2`))
  (`LightComponent.SetIntensity` _pointlight2 (`self.Brightness`))
  (`LightComponent.SetLightColor` _pointlight2 (`self.Color`) true)
  (`SpotLightComponent.SetInnerConeAngle` _pointlight2 (`self.Inner Cone Angle`))
  (`SpotLightComponent.SetOuterConeAngle` _pointlight2 (`self.Outer Cone Angle`))
  (set `self.MaxBrightness` (`self.Brightness`)))