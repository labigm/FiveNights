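; Ceiling bar light fixture built from five point lights that share one look and can be dimmed together.
; The construction script applies the Brightness, Color and SourceRadius variables to all five lights.
; DimLights adds a signed Amount to Brightness, clamps it between MinLight and MaxLight, and pushes the new intensity to every light.
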(fn `Dim Lights`
  (params (amount :type "Float (double-precision)"))
  (bind _brightness (`self.Brightness`))
  (if (or (> _brightness (`self.Min Light`)) (< _brightness (`self.Max Light`)))
    (set `self.Brightness` (+ amount (`self.Brightness`)))
    (if (> (`self.Brightness`) (`self.Max Light`))
      (set `self.Brightness` (`self.Max Light`))
      (elif (< (`self.Brightness`) (`self.Min Light`))
        (set `self.Brightness` (`self.Min Light`))))
    (`LightComponent.SetIntensity` (`self.PointLight1`) (`self.Brightness`))
    (`LightComponent.SetIntensity` (`self.PointLight2`) (`self.Brightness`))
    (`LightComponent.SetIntensity` (`self.PointLight3`) (`self.Brightness`))
    (`LightComponent.SetIntensity` (`self.PointLight4`) (`self.Brightness`))
    (`LightComponent.SetIntensity` (`self.PointLight5`) (`self.Brightness`))
    (return)
    (else
      (return))))

(fn `UserConstructionScript`
  (bind _pointlight1 (`self.PointLight1`))
  (bind _pointlight3 (`self.PointLight3`))
  (bind _pointlight5 (`self.PointLight5`))
  (bind _pointlight4 (`self.PointLight4`))
  (bind _pointlight2 (`self.PointLight2`))
  (`LightComponent.SetIntensity` _pointlight1 (`self.Brightness`))
  (`LightComponent.SetLightColor` _pointlight1 (`self.Color`) true)
  (`PointLightComponent.SetSourceRadius` _pointlight1 (`self.Source Radius`))
  (`LightComponent.SetIntensity` _pointlight2 (`self.Brightness`))
  (`LightComponent.SetLightColor` _pointlight2 (`self.Color`) true)
  (`PointLightComponent.SetSourceRadius` _pointlight2 (`self.Source Radius`))
  (`LightComponent.SetIntensity` _pointlight3 (`self.Brightness`))
  (`LightComponent.SetLightColor` _pointlight3 (`self.Color`) true)
  (`PointLightComponent.SetSourceRadius` _pointlight3 (`self.Source Radius`))
  (`LightComponent.SetIntensity` _pointlight4 (`self.Brightness`))
  (`LightComponent.SetLightColor` _pointlight4 (`self.Color`) true)
  (`PointLightComponent.SetSourceRadius` _pointlight4 (`self.Source Radius`))
  (`LightComponent.SetIntensity` _pointlight5 (`self.Brightness`))
  (`LightComponent.SetLightColor` _pointlight5 (`self.Color`) true)
  (`PointLightComponent.SetSourceRadius` _pointlight5 (`self.Source Radius`)))