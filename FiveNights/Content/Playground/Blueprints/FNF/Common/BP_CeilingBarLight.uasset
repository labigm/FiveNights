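; BP_CeilingBarLight is a ceiling bar light fixture built from three point lights.
; Its construction script applies shared Brightness, Color and SourceRadius values to all three lights.
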(fn `UserConstructionScript`
  (bind _pointlight1 (`self.PointLight1`))
  (bind _pointlight3 (`self.PointLight3`))
  (bind _pointlight2 (`self.PointLight2`))
  (`LightComponent.SetIntensity` _pointlight1 (`self.Brightness`))
  (`LightComponent.SetLightColor` _pointlight1 (`self.Color`) true)
  (`PointLightComponent.SetSourceRadius` _pointlight1 (`self.Source Radius`))
  (`LightComponent.SetIntensity` _pointlight2 (`self.Brightness`))
  (`LightComponent.SetLightColor` _pointlight2 (`self.Color`) true)
  (`PointLightComponent.SetSourceRadius` _pointlight2 (`self.Source Radius`))
  (`LightComponent.SetIntensity` _pointlight3 (`self.Brightness`))
  (`LightComponent.SetLightColor` _pointlight3 (`self.Color`) true)
  (`PointLightComponent.SetSourceRadius` _pointlight3 (`self.Source Radius`)))